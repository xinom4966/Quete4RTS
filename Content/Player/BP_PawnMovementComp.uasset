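; Movement component for BP_CameraPawn that slides the camera pawn along its local X and Y axes from axis input.
; On init it caches the owning pawn, and BasicMovementControls applies swept local offsets scaled by default speed and a modifier.
; As wired, enabled movement requires both axes to be non-zero, while the DisableCameraMovement branch still moves on one axis, X taking priority.
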(event Custom|InitComponent
  (bind _asbp_camera_pawn (Utilities|Casting|CastToBP_CameraPawn (Components|GetOwner)))
  (Variables|References|SetCameraPawnRef _asbp_camera_pawn))

(event EventBeginPlay)

(event EventTick
  (params (DeltaSeconds :type Float%20%28single-precision%29)))

(fn BasicMovementControls
  (params (AxisValueX :type Float%20%28double-precision%29) (AxisValueY :type Float%20%28double-precision%29))
  (LocalVariables|SetAxisValueXLocal AxisValueX)
  (LocalVariables|SetAxisValueYLocal AxisValueY)
  (if (not (Variables|Movement|bools|GetbDisableCameraMovement))
    (if (and (!= (LocalVariables|GetAxisValueXLocal) 0.0) (!= (LocalVariables|GetAxisValueYLocal) 0.0))
      (Transformation|AddActorLocalOffset (Variables|References|GetCameraPawnRef) (+ (Math|Vector|MakeVector (* (LocalVariables|GetAxisValueXLocal) (Variables|Movement|Settings|GetDefaultMovementSpeed) (Variables|Movement|Settings|GetMovementSpeedModifier)) 0.0 0.0) (Math|Vector|MakeVector 0.0 (* (LocalVariables|GetAxisValueYLocal) (Variables|Movement|Settings|GetDefaultMovementSpeed) (Variables|Movement|Settings|GetMovementSpeedModifier)) 0.0)) true false))
    (elif (!= (LocalVariables|GetAxisValueXLocal) 0.0)
      (Transformation|AddActorLocalOffset (Variables|References|GetCameraPawnRef) (Math|Vector|MakeVector (* (LocalVariables|GetAxisValueXLocal) (Variables|Movement|Settings|GetDefaultMovementSpeed) (Variables|Movement|Settings|GetMovementSpeedModifier)) 0.0 0.0) true false)
      (elif (!= (LocalVariables|GetAxisValueYLocal) 0.0)
        (Transformation|AddActorLocalOffset (Variables|References|GetCameraPawnRef) (Math|Vector|MakeVector 0.0 (* (LocalVariables|GetAxisValueYLocal) (Variables|Movement|Settings|GetDefaultMovementSpeed) (Variables|Movement|Settings|GetMovementSpeedModifier)) 0.0) true false)))))